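; BP_Unit is a grid-based unit that walks tile paths, holds HP and attack stats, and shows HP and active bar widgets.
; Construction loads data for its unit type, setting the Paper child-actor character, PaperZD animation instance and stats.
; Movement chains a timeline per tile, adding a jump arc on height changes, switching animation states and broadcasting walk events.
; SubtractHP updates the bar on survival and returns true when HP reaches zero.
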(event Custom|Event%20FollowPath
  (params (Path :type Array%20of%20Int%20Point%20Structures))
  (if (> (Utilities|Array|Length Path) 0)
    (Variables|Default|SetCurrentPathToFollow Path)
    (Default|CallOnUnitStartedWalking self)
    (CallFunction|ContinuetoFollowPath)))

(event Custom|ContinueToFollowPath
  (bind _timeline_unitmovement (Variables|Default|GetTimeline_UnitMovement))
  (if (> (Utilities|Array|Length (Variables|Default|GetCurrentPathToFollow)) 0)
    (CallFunction|SetAnimationState "NewEnumerator1")
    (Variables|Default|SetPreviousTransform (Transformation|GetActorTransform))
    (Variables|Default|SetNextTransform (Math|Transform|MakeTransform (.location (Utilities|Struct|BreakS_TileData (.Value (Utilities|Map|Find (Variables|/Game/Dynamic/Blueprints/Core/Grid/BP_Grid.BP_Grid_C|GetGridTiles (Variables|Default|GetGrid)) (Utilities|Array|Get(acopy) (Variables|Default|GetCurrentPathToFollow)))))) "0, 0, 0" "1.000000,1.000000,1.000000"))
    (Components|Timeline|SetPlayRate _timeline_unitmovement (/ (Components|Timeline|GetTimelineLength _timeline_unitmovement) (Variables|Default|GetMoveTimePerTile)))
    (bind (_direction _locationalpha _jump) (Timeline|Timeline_UnitMovement PlayFromStart)
      (:Update
        (Transformation|SetActorLocation (+ (Math|Vector|Lerp(Vector) (.location (Variables|Default|GetPreviousTransform)) (.location (Variables|Default|GetNextTransform)) _locationalpha) (Math|Vector|MakeVector 0.0 0.0 (select (Math|Float|NearlyEqual(Float) (.z (.location (Variables|Default|GetPreviousTransform))) (.z (.location (Variables|Default|GetNextTransform))) 5.0) 0.0 _jump))) false false))
      (:Finished
        (Default|CallOnReachedNewTile self (Utilities|Array|Get(acopy) (Variables|Default|GetCurrentPathToFollow)))
        (Utilities|Array|RemoveIndex (Variables|Default|GetCurrentPathToFollow))
        (CallFunction|ContinuetoFollowPath)))
    (else
      (CallFunction|SetAnimationState "NewEnumerator0")
      (Default|CallOnFinishedWalking self)
      (Variables|Default|SetHasMoved true))))

(event EventBeginPlay
  (CallFunction|SetAnimationState "NewEnumerator0")
  (bind _output_get (Variables|Default|SetHpBar (CallFunction|GetHpBar)))
  (Default|EventSetUnit _output_get self)
  (bind _output_get_2 (Variables|Default|SetActiveBar (CallFunction|GetActiveBar)))
  (Default|EventSetUnit _output_get_2 self))

(fn ConstructionScript
  (bind _unitdata (CallFunction|GetDefaultUnitDatafromUnitType (Variables|Default|GetUnitType)))
  (CallFunction|SetUnitData _unitdata))

(fn SetIsHovered
  (params (Hovered :type Boolean))
  (Variables|Default|SetIsHovered Hovered))

(fn SetIsSelected
  (params (Selected :type Boolean))
  (Variables|Default|SetIsSelected Selected))

(fn SetIndex
  (bind _returnvalue (Transformation|GetActorLocation))
  (bind _values (Utilities|Map|Values (Variables|/Game/Dynamic/Blueprints/Core/Grid/BP_Grid.BP_Grid_C|GetGridTiles (Variables|Default|GetGrid))))
  (for _array_element _values
    (if (and (== (.x _returnvalue) (.x (.location (.Transform (Utilities|Struct|BreakS_TileData _array_element))))) (== (.y _returnvalue) (.y (.location (.Transform (Utilities|Struct|BreakS_TileData _array_element))))))
      (Variables|Default|SetIndex (.Index (Utilities|Struct|BreakS_TileData _array_element)))
      (return)))
  (Variables|Default|SetIndex (Utilities|Struct|MakeIntPoint -9999 -9999))
  (return))

(fn SetUnitData
  (params (Data :type S%20Unit%20Data%20Structure%20%28by%20ref%29))
  (bind _output_get (Variables|Default|SetUnitData Data))
  (ChildActorComponent|SetChildActorClass (Variables|Default|GetChildActor_Character) (.PaperBp (Utilities|Struct|BreakS_UnitDataAssets (.Assets (Utilities|Struct|BreakS_UnitData _output_get)))))
  (Class|PaperZDAnimationComponent|SetAnimInstanceClass (Variables|Default|GetPaperZDAnimation) (.AnimBp (Utilities|Struct|BreakS_UnitDataAssets (.Assets (Utilities|Struct|BreakS_UnitData _output_get)))))
  (Variables|Default|SetHPCurrent (.HP_Max (Utilities|Struct|BreakS_UnitData_Stats (.Stats (Utilities|Struct|BreakS_UnitData _output_get)))))
  (Variables|Default|SetAttack (.Attack (Utilities|Struct|BreakS_UnitData_Stats (.Stats (Utilities|Struct|BreakS_UnitData _output_get))))))

(fn SetGrid
  (params (Grid :type BP%20Grid%20Object%20Reference))
  (Variables|Default|SetGrid Grid))

(fn SubtractHP
  (params (Damage :type Integer))
  (if (> (- (Variables|Default|GetHPCurrent) Damage) 0)
    (Variables|Default|SetHPCurrent (- (Variables|Default|GetHPCurrent) Damage))
    (Default|EventUpdateHpBar (CallFunction|GetHpBar))
    (return false)
    (else
      (Variables|Default|SetHPCurrent 0)
      (return true))))

(fn SetAnimationState
  (params (State :type E_UnitAnimationState%20Enum :default "NewEnumerator0"))
  (Class|BPIUnitAnimation|SetUnitAnimationState(Message) (Variables|/Script/PaperZD.PaperZDAnimationComponent|GetAnimInstance (Variables|Default|GetPaperZDAnimation)) State))

(fn GetHpBar
  (return (.AsW%20Hp%20Bar (Utilities|Casting|CastToW_HpBar (UserInterface|GetUserWidgetObject (Variables|Default|GetWidget_HpBar))))))

(fn GetActiveBar
  (bind _asw_active_bar (Utilities|Casting|CastToW_ActiveBar (UserInterface|GetUserWidgetObject (Variables|Default|GetWidget_ActiveBar))))
  (return _asw_active_bar))